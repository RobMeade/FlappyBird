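; BP_SaveGame is a save game object that persists the player's best score in a named slot.
; Initialise sets the score in memory, while SaveData sets it and writes the object to the slot.
; LoadData copies the score from the saved object into itself and returns it, or saves itself to create the slot when none exists and returns its current value.
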(fn Initialise
  (params (BestScore :type Integer))
  ;[1 1 1] Initialise
  (Variables|Default|SetBestScore BestScore))

(fn LoadData
  ;[1 1 1] Load Data
  (bind _returnvalue (SaveGame|DoesSaveGameExist (Variables|Default|GetSlotName)))
  (if _returnvalue
    (bind _returnvalue_2 (SaveGame|LoadGamefromSlot (Variables|Default|GetSlotName)))
    (bind _asbp_save_game (Utilities|Casting|CastToBP_SaveGame _returnvalue_2))
    (Variables|Default|SetBestScore (Variables|BP_SaveGame_C|GetBestScore _asbp_save_game))
    (else
      (SaveGame|SaveGametoSlot self (Variables|Default|GetSlotName))))
  (return (Variables|Default|GetBestScore)))

(fn SaveData
  (params (BestScore :type Integer))
  ;[1 1 1] Save Data
  (Variables|Default|SetBestScore BestScore)
  (SaveGame|SaveGametoSlot self (Variables|Default|GetSlotName)))
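; Game mode for a Flappy Bird-style game that owns the game state and game speed, broadcasting each state change through a GameStateChanged dispatcher.
; On BeginPlay it binds to UI click events from the player controller and to the bird's initialised and died events, which drive the state transitions.
; Pipes passed to RegisterPipe report reaching their target location, which increments the player controller's score.
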(event EventEndPlay
  (params (EndPlayReason :type EEndPlayReason%20Enum :default "Destroyed"))
  ;[1 1 1] Finalise
  (CallFunction|UnbindAllEvents))

(event EventBeginPlay
  ;[1 1 1] Initialise
  (CallFunction|SetReferences)
  (CallFunction|BindtoEvents))

(fn ConstructionScript)

(fn BindtoEvents
  ;[1 1 1] Bind to Events
  (EventDispatchers|BindEventtoMainMenuPlayButtonClicked (Variables|Default|Get_PlayerController) (EventDispatchers|CreateEvent :!event OnMainMenuPlayButtonClicked))
  (EventDispatchers|BindEventtoGetReadyClicked (Variables|Default|Get_PlayerController) (EventDispatchers|CreateEvent :!event OnGetReadyClicked))
  (EventDispatchers|BindEventtoGameOverPlayButtonClicked (Variables|Default|Get_PlayerController) (EventDispatchers|CreateEvent :!event OnGameOverPlayButtonClicked))
  (bind _asbp_bird (Utilities|Casting|CastToBP_Bird (Game|Player|GetPlayerPawn 0)))
  (EventDispatchers|BindEventtoBirdDied _asbp_bird (EventDispatchers|CreateEvent :!event OnBirdDied))
  (bind _asbp_bird_2 (Utilities|Casting|CastToBP_Bird (Game|Player|GetPlayerPawn 0)))
  (EventDispatchers|BindEventtoInitialised _asbp_bird_2 (EventDispatchers|CreateEvent :!event OnPlayerPawnInitialised)))

(fn GameOver
  ;[1 1 1] Game Over
  (bind _output_get (Variables|Default|Set_GameState "NewEnumerator3"))
  (Default|CallGameStateChanged _output_get))

(fn GetGameSpeed
  ;[1 1 1] Get Game Speed
  (return (Variables|Default|Get_GameSpeed)))

(fn OnBirdDied
  ;[1 1 1] Bird Died
  (CallFunction|GameOver))

(fn OnGameOverPlayButtonClicked
  ;[1 1 1] Game Over Play Button Clicked
  (bind _output_get (Variables|Default|Set_GameState "NewEnumerator1"))
  (Default|CallGameStateChanged _output_get))

(fn OnGetReadyClicked
  ;[1 1 1] Get Ready Clicked
  (bind _output_get (Variables|Default|Set_GameState "NewEnumerator2"))
  (Default|CallGameStateChanged _output_get))

(fn OnMainMenuPlayButtonClicked
  ;[1 1 1] Main Menu Play Button Clicked
  (bind _output_get (Variables|Default|Set_GameState "NewEnumerator1"))
  (Default|CallGameStateChanged _output_get))

(fn OnPipeTargetLocationReached
  ;[1 1 1] Pipe Target Location Reached
  (Default|IncrementScore (Variables|Default|Get_PlayerController)))

(fn OnPlayerPawnInitialised
  ;[1 1 1] Player Pawn Initialised
  (CallFunction|StartGame))

(fn RegisterPipe
  (params (Pipe :type BP%20Pipe%20Object%20Reference))
  ;[1 1 1] Register Pipe
  (EventDispatchers|BindEventtoTargetLocationReached Pipe (EventDispatchers|CreateEvent :!event OnPipeTargetLocationReached)))

(fn SetReferences
  ;[1 1 1] Set References
  (bind _asbp_player_controller (Utilities|Casting|CastToBP_PlayerController (Game|GetPlayerController 0)))
  (Variables|Default|Set_PlayerController _asbp_player_controller))

(fn StartGame
  ;[1 1 1] Start Game
  (Variables|Default|Set_GameSpeed (Variables|Default|Get_DefaultGameSpeed))
  (bind _output_get (Variables|Default|Set_GameState "NewEnumerator0"))
  (Default|CallGameStateChanged _output_get))

(fn UnbindAllEvents
  ;[1 1 1] Unbind All Events
  (EventDispatchers|UnbindallEventsfromGameStateChanged))
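; Player controller for a Flappy Bird-style game that owns the UI, score and saved best score.
; On begin play it loads the save, creates the menu, get-ready, HUD and game-over widgets, and binds to the game mode and bird.
; Game-state changes toggle widgets, input mode and flap input; bird grounding saves any new best and shows game over.
; Widget clicks are re-broadcast through its own event dispatchers.
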(event EventBeginPlay
  ;[1 1 1] Initialise
  (CallFunction|Initialise))

(event EventEndPlay
  (params (EndPlayReason :type EEndPlayReason%20Enum :default "Destroyed"))
  ;[1 1 1] Finalise
  (CallFunction|UnbindAllEvents))

(event Input|ActionEvents|InputActionFlap
  (params (Key :type Key%20Structure :default "None"))
  ;[1 1 1] Player Interaction
  (:Pressed
    (CallFunction|Flap)))

(fn ConstructionScript)

(fn BindtoUIEvents
  ;[1 1 1] Bind to UI Events
  (EventDispatchers|BindEventtoPlayButtonClicked (Variables|References|Get_MainMenu) (EventDispatchers|CreateEvent :!event OnMainMenuPlayButtonClicked))
  (EventDispatchers|BindEventtoGetReadyClicked (Variables|References|Get_GetReady) (EventDispatchers|CreateEvent :!event OnGetReadyClicked))
  (EventDispatchers|BindEventtoGameOverPlayButtonClicked (Variables|References|Get_GameOver) (EventDispatchers|CreateEvent :!event OnGameOverPlayButtonClicked)))

(fn CreateUIWidgets
  ;[1 1 1] Create UI Widgets
  (bind _returnvalue (UserInterface|CreateWidget "/Game/UI/WBP_MainMenu.WBP_MainMenu_C" self))
  (bind _output_get (Variables|References|Set_MainMenu _returnvalue))
  (UserInterface|Viewport|AddtoViewport _output_get 0)
  (Widget|SetVisibility (Variables|References|Get_MainMenu) "Hidden")
  (bind _returnvalue_2 (UserInterface|CreateWidget "/Game/UI/WBP_GetReady.WBP_GetReady_C" self))
  (bind _output_get_2 (Variables|References|Set_GetReady _returnvalue_2))
  (UserInterface|Viewport|AddtoViewport _output_get_2 1)
  (Widget|SetVisibility (Variables|References|Get_GetReady) "Hidden")
  (bind _returnvalue_3 (UserInterface|CreateWidget "/Game/UI/WBP_HUD.WBP_HUD_C" self))
  (bind _output_get_3 (Variables|References|Set_HUD _returnvalue_3))
  (UserInterface|Viewport|AddtoViewport _output_get_3 0)
  (Widget|SetVisibility (Variables|References|Get_HUD) "Hidden")
  (bind _returnvalue_4 (UserInterface|CreateWidget "/Game/UI/WBP_GameOver.WBP_GameOver_C" self))
  (bind _output_get_4 (Variables|References|Set_GameOver _returnvalue_4))
  (UserInterface|Viewport|AddtoViewport _output_get_4 0)
  (Widget|SetVisibility (Variables|References|Get_GameOver) "Hidden"))

(fn Flap
  ;[1 1 1] Flap
  (if (Variables|Default|Get_InputEnabled)
    (Default|Flap (Variables|References|Get_Pawn))))

(fn IncrementScore
  ;[1 1 1] Increment Score
  (bind _result (Math|Integer|IncrementInt (Variables|Default|Get_Score))
    (:%20%20
      (Default|SetScore (Variables|References|Get_HUD) _result))))

(fn Initialise
  ;[1 1 1] Initialise
  (bind _returnvalue (SaveGame|CreateSaveGameObject "/Game/Core/BP_SaveGame.BP_SaveGame_C"))
  (bind _output_get (Variables|References|Set_SaveGame _returnvalue))
  (bind _bestscore (Default|LoadData _output_get))
  (Variables|Default|Set_BestScore _bestscore)
  (bind _asbp_game_mode (Utilities|Casting|CastToBP_GameMode (Game|GetGameMode)))
  (EventDispatchers|BindEventtoGameStateChanged _asbp_game_mode (EventDispatchers|CreateEvent :!event OnGameStateChanged))
  (bind _asbp_bird (Utilities|Casting|CastToBP_Bird (Game|Player|GetPlayerPawn 0)))
  (bind _output_get_2 (Variables|References|Set_Pawn _asbp_bird))
  (EventDispatchers|BindEventtoBirdGrounded _output_get_2 (EventDispatchers|CreateEvent :!event OnBirdGrounded))
  (CallFunction|CreateUIWidgets)
  (CallFunction|BindtoUIEvents))

(fn ResetScore
  ;[1 1 1] Reset Score
  (bind _output_get (Variables|Default|Set_Score 0))
  (Default|SetScore (Variables|References|Get_HUD) _output_get))

(fn OnBirdGrounded
  ;[1 1 1] Bird Grounded
  (CallFunction|IsNewBestScore)
  (Default|SetScore (Variables|References|Get_GameOver) (Variables|Default|Get_Score) (Variables|Default|Get_BestScore) (Variables|Default|Get_NewBestScore))
  (Widget|SetVisibility (Variables|References|Get_GameOver) "Visible")
  (Widget|SetVisibility (Variables|References|Get_HUD) "Hidden")
  (Input|SetInputModeUIOnly self (Variables|References|Get_MainMenu) "DoNotLock")
  (Variables|Default|SetbShowMouseCursor true))

(fn OnGameGetReady
  ;[1 1 1] Game - Get Ready
  (Widget|SetVisibility (Variables|References|Get_MainMenu) "Hidden")
  (Widget|SetVisibility (Variables|References|Get_GameOver) "Hidden")
  (Widget|SetVisibility (Variables|References|Get_GetReady) "Visible")
  (Widget|SetVisibility (Variables|References|Get_HUD) "Visible")
  (CallFunction|ResetScore))

(fn OnGameOver
  ;[1 1 1] Game - Over
  (Variables|Default|Set_InputEnabled false))

(fn OnGamePlaying
  ;[1 1 1] Game - Playing
  (Variables|Default|Set_InputEnabled true)
  (Widget|SetVisibility (Variables|References|Get_GetReady) "Hidden")
  (Input|SetInputModeGameOnly self)
  (Variables|Default|SetbShowMouseCursor false))

(fn OnGameStarted
  ;[1 1 1] Game - Started
  (Widget|SetVisibility (Variables|References|Get_MainMenu) "Visible")
  (Input|SetInputModeUIOnly self (Variables|References|Get_MainMenu) "DoNotLock")
  (Variables|Default|SetbShowMouseCursor true))

(fn OnGameOverPlayButtonClicked
  ;[1 1 1] Game Over Play Button Clicked
  (Default|CallGameOverPlayButtonClicked))

(fn OnGameStateChanged
  (params (GameState :type EGameState%20Enum :default "NewEnumerator0"))
  ;[1 1 1] Game State Changed
  (switch Utilities|FlowControl|Switch|SwitchonEGameState GameState
    (:NewEnumerator0
      (EventHandlers|OnGameStarted))
    (:NewEnumerator1
      (EventHandlers|OnGameGetReady))
    (:NewEnumerator2
      (EventHandlers|OnGamePlaying))
    (:NewEnumerator3
      (EventHandlers|OnGameOver))))

(fn OnGetReadyClicked
  ;[1 1 1] Get Ready Clicked
  (Default|CallGetReadyClicked))

(fn OnMainMenuPlayButtonClicked
  ;[1 1 1] Main Menu Play Button Clicked
  (Default|CallMainMenuPlayButtonClicked))

(fn UnbindAllEvents
  ;[1 1 1] Unbind All Events
  (EventDispatchers|UnbindallEventsfromMainMenuPlayButtonClicked)
  (EventDispatchers|UnbindallEventsfromGetReadyClicked)
  (EventDispatchers|UnbindallEventsfromGameOverPlayButtonClicked))

(fn IsNewBestScore
  ;[1 1 1] Is New Best Score
  (bind _output_get (Variables|Default|Set_NewBestScore (> (Variables|Default|Get_Score) (Variables|Default|Get_BestScore))))
  (if _output_get
    (Variables|Default|Set_BestScore (Variables|Default|Get_Score))
    (Default|SaveData (Variables|References|Get_SaveGame) (Variables|Default|Get_BestScore)))
  (return (Variables|Default|Get_NewBestScore)))
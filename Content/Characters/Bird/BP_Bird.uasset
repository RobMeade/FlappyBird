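; BP_Bird is the Flappy Bird-style character, a flipbook bird with randomised colour.
; BP_GameMode state changes reset it into timeline-driven bobbing for menu and get-ready, then enable physics for play.
; Flap zeroes velocity before applying an upward impulse, and Tick pauses the wing animation on select frames while falling.
; Overlaps kill it, while hits also snap it onto the ground, broadcasting died and grounded events with one-shot death sounds.
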(event OnComponentHit(Bird)
  (params (HitComponent :type Primitive%20Component%20Object%20Reference) (OtherActor :type Actor%20Object%20Reference) (OtherComp :type Primitive%20Component%20Object%20Reference) (NormalImpulse :type Vector :default "0, 0, 0") (Hit :type Hit%20Result%20Structure%20%28by%20ref%29))
  ;[1 1 1] Ground
  (CallFunction|Ground (.HitComponent (Collision|BreakHitResult Hit)))
  (CallFunction|PlayDeathSFX false))

(event OnComponentBeginOverlap(Bird)
  (params (OverlappedComponent :type Primitive%20Component%20Object%20Reference) (OtherActor :type Actor%20Object%20Reference) (OtherComp :type Primitive%20Component%20Object%20Reference) (OtherBodyIndex :type Integer) (bFromSweep :type Boolean) (SweepResult :type Hit%20Result%20Structure%20%28by%20ref%29))
  ;[1 1 1] Die
  (CallFunction|Die)
  (CallFunction|PlayDeathSFX true))

(event Custom|Flap
  ;[1 1 1] Flap
  (CallFunction|ApplyFlapForce)
  (CallFunction|PlayFlapSFX))

(event Custom|StartAutoFlight
  ;[1 1 1] Auto Flight
  (bind _flightalpha (Timeline|Fly PlayFromStart)
    (:Update
      (CallFunction|SetAutoFlightLocation _flightalpha))))

(event Custom|StopAutoFlight
  ;[1 1 1] Auto Flight
  (bind _flightalpha (Timeline|Fly Stop)
    (:Update
      (CallFunction|SetAutoFlightLocation _flightalpha))))

(event EventBeginPlay
  ;[1 1 1] Initialise
  (Utilities|FlowControl|Delay 0.2)
  (CallFunction|Initialise))

(event EventEndPlay
  (params (EndPlayReason :type EEndPlayReason%20Enum :default "Destroyed"))
  ;[1 1 1] Finalise
  (CallFunction|UnbindAllEvents))

(event EventTick
  (params (DeltaSeconds :type Float%20%28single-precision%29))
  ;[1 1 1] Tick
  (if (CallFunction|IsFalling)
    (CallFunction|PauseFlapAnimation)
    (else
      (CallFunction|UnpauseFlapAnimation))))

(fn ConstructionScript)

(fn OnGameGetReady
  ;[1 1 1] Game - Get Ready
  (Variables|Default|Set_AutoFlightOrigin (Variables|Default|Get_GetReadyOrigin))
  (CallFunction|Reset (Variables|Default|Get_GetReadyOrigin))
  (CallFunction|SetBirdFlipbook))

(fn OnGameOver
  ;[1 1 1] Game - Over
  (CallFunction|SetRandomBirdColour))

(fn OnGamePlaying
  ;[1 1 1] Game - Playing
  (Variables|Default|Set_AutoFlightOrigin (Variables|Default|Get_GetReadyOrigin))
  (CallFunction|StopAutoFlight)
  (Physics|SetSimulatePhysics (Variables|Default|GetBird) true))

(fn OnGameStarted
  ;[1 1 1] Game - Started
  (Variables|Default|Set_AutoFlightOrigin (Variables|Default|Get_MainMenuOrigin))
  (CallFunction|Reset (Variables|Default|Get_MainMenuOrigin))
  (CallFunction|SetRandomBirdColour)
  (CallFunction|SetBirdFlipbook))

(fn OnGameStateChanged
  (params (GameState :type EGameState%20Enum :default "NewEnumerator0"))
  ;[1 1 1] Game State Changed
  (switch Utilities|FlowControl|Switch|SwitchonEGameState GameState
    (:NewEnumerator0
      (EventHandlers|OnGameStarted))
    (:NewEnumerator1
      (EventHandlers|OnGameGetReady))
    (:NewEnumerator2
      (EventHandlers|OnGamePlaying))
    (:NewEnumerator3
      (EventHandlers|OnGameOver))))

(fn ApplyFlapForce
  ;[1 1 1] Apply Flap Force
  (Physics|SetPhysicsLinearVelocity (Variables|Default|GetBird) "0, 0, 0" false "None")
  (Physics|AddImpulse (Variables|Default|GetBird) (Variables|Default|Get_FlapImpulse) "None" true))

(fn Die
  ;[1 1 1] Die
  (if (not (Variables|Default|Get_IsDead))
    (Variables|Default|Set_IsDead true)
    (Default|CallBirdDied)))

(fn GetGroundedLocation
  (params (Base :type Primitive%20Component%20Object%20Reference%20%28by%20ref%29))
  ;[1 1 1] Get Grounded Location
  (return (+ (.z (Transformation|GetWorldLocation Base)) (.z (.BoxExtent (Collision|GetComponentBounds Base))) (.z (.BoxExtent (Collision|GetComponentBounds (Variables|Default|GetBird)))))))

(fn Ground
  (params (Base :type Primitive%20Component%20Object%20Reference%20%28by%20ref%29))
  ;[1 1 1] Ground
  (if (not (Variables|Default|Get_IsGrounded))
    (Physics|SetSimulatePhysics (Variables|Default|GetBird) false)
    (Utilities|FlowControl|Sequence
      (:then_0
        (if (not (Variables|Default|Get_IsDead))
          (CallFunction|Die)))
      (:then_1
        (Transformation|SetWorldRotation (Variables|Default|GetBird) "0, 0, 0" false false)
        (Transformation|SetWorldLocation (Variables|Default|GetBird) (Math|Vector|MakeVector -55.0 0.0 (CallFunction|GetGroundedLocation Base)) false false)
        (Variables|Default|Set_IsGrounded true)
        (Default|CallBirdGrounded)))))

(fn Initialise
  ;[1 1 1] Initialise
  (bind _asbp_game_mode (Utilities|Casting|CastToBP_GameMode (Game|GetGameMode)))
  (EventDispatchers|BindEventtoGameStateChanged _asbp_game_mode (EventDispatchers|CreateEvent :!event OnGameStateChanged))
  (Variables|Default|Set_FlapImpulse "0, 0,331.299988")
  (Default|CallInitialised))

(fn PlayDeathSFX
  (params (WithFall :type Boolean))
  ;[1 1 1] Play Death SFX
  (if (not (Variables|Default|Get_HasDeathSFXPlayed))
    (Variables|Default|Set_HasDeathSFXPlayed true)
    (Audio|PlaySound2D "/Game/Characters/Bird/Audio/A_Die_Cue.A_Die_Cue" 1.0 1.0 0.0 0 0)
    (if WithFall
      (Audio|PlaySound2D "/Game/Characters/Bird/Audio/A_Fall_Cue.A_Fall_Cue" 1.0 1.0 0.0 0 0))))

(fn PlayFlapSFX
  ;[1 1 1] Play Flap SFX
  (Audio|PlaySound2D "/Game/Characters/Bird/Audio/A_Flap_Cue.A_Flap_Cue" 1.0 1.0 0.0 0 0))

(fn Reset
  (params (Location :type Vector))
  ;[1 1 1] Reset
  (Variables|Default|Set_IsDead false)
  (Variables|Default|Set_IsGrounded false)
  (Variables|Default|Set_HasDeathSFXPlayed false)
  (Transformation|SetWorldLocation (Variables|Default|GetBird) Location false true)
  (Components|Timeline|PlayfromStart (Variables|Default|GetBird))
  (CallFunction|StartAutoFlight))

(fn SetBirdFlipbook
  ;[1 1 1] Set Bird Flipbook
  (Sprite|SetFlipbook (Variables|Default|GetBird) (Utilities|Select :Index (Variables|Default|Get_BirdColour) :NewEnumerator0 "/Game/Characters/Bird/Animation/PFB_Bird_Blue_Flap.PFB_Bird_Blue_Flap" :NewEnumerator1 "/Game/Characters/Bird/Animation/PFB_Bird_Red_Flap.PFB_Bird_Red_Flap" :NewEnumerator2 "/Game/Characters/Bird/Animation/PFB_Bird_Yellow_Flap.PFB_Bird_Yellow_Flap"))
  (Components|Timeline|SetPlayRate (Variables|Default|GetBird) 1.0))

(fn SetRandomBirdColour
  ;[1 1 1] Set Random Bird Colour
  (Variables|Default|Set_BirdColour (Utilities|Enum|ByteToEnumEBirdColour (Math|Conversions|ToByte(Integer) (Math|Random|RandomIntegerinRange 0 (- (|GetNumEnumEntries) 1))))))

(fn SetAutoFlightLocation
  (params (FlightAlpha :type Float%20%28single-precision%29))
  (bind __autoflightorigin (Variables|Default|Get_AutoFlightOrigin))
  (bind __autoflightorigin_2 (Variables|Default|Get_AutoFlightOrigin))
  ;[1 1 1] Set Auto Flight Location
  (Transformation|SetWorldLocation (Variables|Default|GetBird) (Math|Vector|MakeVector (.x __autoflightorigin) (.y __autoflightorigin) (Math|Float|Lerp (+ (.z __autoflightorigin_2) (+ (Variables|Default|Get_AutoFlightMinimumElevation) (Variables|Default|Get_AutoFlightMaximumElevation))) (+ (.z __autoflightorigin_2) (Variables|Default|Get_AutoFlightMinimumElevation)) FlightAlpha)) false false))

(fn UnbindAllEvents
  ;[1 1 1] Unbind All Events
  (EventDispatchers|UnbindallEventsfromBirdDied)
  (EventDispatchers|UnbindallEventsfromBirdGrounded)
  (EventDispatchers|UnbindallEventsfromInitialised))

(fn IsFalling
  ;[1 1 1] Is Falling?
  (return (<= (.z (Transformation|GetComponentVelocity (Variables|Default|GetBird))) 0.0)))

(fn UnpauseFlapAnimation
  (if (Variables|Default|Get_IsFlapAnimationPaused)
    (Components|Timeline|SetPlayRate (Variables|Default|GetBird) 1.0)
    (Variables|Default|Set_IsFlapAnimationPaused false)))

(fn PauseFlapAnimation
  (bind _bird (Variables|Default|GetBird))
  (bind _returnvalue (Class|PaperFlipbookComponent|GetPlaybackPositioninFrames _bird))
  (if (and (or (== _returnvalue 0) (== _returnvalue 2)) (not (Variables|Default|Get_IsFlapAnimationPaused)))
    (Components|Timeline|SetPlayRate (Variables|Default|GetBird) 0.0)
    (Variables|Default|Set_IsFlapAnimationPaused true)))
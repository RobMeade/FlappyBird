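; Scrolling pipe obstacle that recycles itself, moving along negative X while the game is in the Playing state.
; It takes its speed from BP_GameMode at BeginPlay and binds to game state changes, which toggle movement.
; Each tick while moving, it checks whether it has passed the left limit, then jumps back to the right with a random height.
; Game Started and Get Ready restore its start location with a new random height; Game Over freezes it.
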(event EventBeginPlay
  ;[1 1 1] Initialise
  (CallFunction|SetSpeed)
  (CallFunction|BindtoEvents))

(event EventTick
  (params (DeltaSeconds :type Float%20%28single-precision%29))
  ;[1 1 1] Tick
  (CallFunction|Move DeltaSeconds))

(fn ConstructionScript)

(fn BindtoEvents
  ;[1 1 1] Bind to Events
  (bind _asbp_game_mode (Utilities|Casting|CastToBP_GameMode (Game|GetGameMode)))
  (EventDispatchers|BindEventtoGameStateChanged _asbp_game_mode (EventDispatchers|CreateEvent :!event OnGameStateChanged)))

(fn Move
  (params (DeltaSeconds :type Float%20%28single-precision%29))
  ;[1 1 1] Move
  (if (Variables|Default|Get_CanMove)
    (Utilities|FlowControl|Sequence
      (:then_0
        (if (CallFunction|ShouldPipeRelocate)
          (CallFunction|Relocate)
          (CallFunction|SetVerticalPosition)))
      (:then_1
        (Transformation|SetWorldLocation (Variables|Default|GetScene) (- (Transformation|GetActorLocation) (Math|Vector|MakeVector (* DeltaSeconds (Variables|Default|Get_Speed)) 0.0 0.0)) false false)))))

(fn Relocate
  ;[1 1 1] Relocate Pipe
  (Transformation|SetActorLocation (Math|Vector|MakeVector 3e+02 (.y (Transformation|GetActorLocation)) 0.0) false false))

(fn Reset
  ;[1 1 1] Reset
  (Transformation|SetActorLocation (Variables|Pipe|GetStartLocation) false false)
  (CallFunction|SetVerticalPosition))

(fn SetSpeed
  ;[1 1 1] Set Speed
  (bind _asbp_game_mode (Utilities|Casting|CastToBP_GameMode (Game|GetGameMode)))
  (Variables|Default|Set_Speed (Default|GetGameSpeed _asbp_game_mode)))

(fn SetVerticalPosition
  (bind _returnvalue (Transformation|GetActorLocation))
  ;[1 1 1] Set Vertical Position
  (Transformation|SetActorLocation (Math|Vector|MakeVector (.x _returnvalue) -1.0 (+ (.z _returnvalue) (Math|Random|RandomFloatinRange -1.1e+02 1.1e+02))) false false))

(fn ShouldPipeRelocate
  ;[1 1 1] Should Pipe Relocate?
  (return (<= (.x (Transformation|GetActorLocation)) -1.5e+02)))

(fn OnGameStateChanged
  (params (GameState :type EGameState%20Enum :default "NewEnumerator0"))
  ;[1 1 1] Game State Changed
  (switch Utilities|FlowControl|Switch|SwitchonEGameState GameState
    (:NewEnumerator0
      (EventHandlers|OnGameStarted))
    (:NewEnumerator1
      (EventHandlers|OnGameGetReady))
    (:NewEnumerator2
      (EventHandlers|OnGamePlaying))
    (:NewEnumerator3
      (EventHandlers|OnGameOver))))

(fn OnGameGetReady
  ;[1 1 1] Game - Get Ready
  (Variables|Default|Set_CanMove false)
  (CallFunction|Reset))

(fn OnGameOver
  ;[1 1 1] Game - Over
  (Variables|Default|Set_CanMove false))

(fn OnGamePlaying
  ;[1 1 1] Game - Playing
  (Variables|Default|Set_CanMove true))

(fn OnGameStarted
  ;[1 1 1] Game - Started
  (Variables|Default|Set_CanMove false)
  (CallFunction|Reset))
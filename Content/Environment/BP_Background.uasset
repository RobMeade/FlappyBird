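; Scrolling 2D Paper2D background actor with a backdrop sprite and a looping base strip.
; Construction aligns the sprites by depth and height, and Tick moves two base sprites along negative X at the GameMode's speed, each jumping behind the other once a full width past the origin.
; GameMode state changes stop scrolling on game over and resume it otherwise, randomly picking a day or night backdrop on start or get ready.
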(event EventTick
  (params (DeltaSeconds :type Float%20%28single-precision%29))
  ;[1 1 1] Tick
  (CallFunction|MoveBases DeltaSeconds))

(event EventBeginPlay
  ;[1 1 1] Initialise
  (CallFunction|SetBaseWidth)
  (CallFunction|SetSpeed)
  (CallFunction|BindtoEvents))

(fn ConstructionScript
  ;[1 1 1] Instantiate
  (CallFunction|AlignPaperSprite (Variables|Default|GetBackground) -2.0)
  (CallFunction|AlignPaperSprite (Variables|Default|GetBase01) 1.0)
  (CallFunction|AlignPaperSprite (Variables|Default|GetBase02) 1.0))

(fn AlignPaperSprite
  (params (Sprite :type Paper%20Sprite%20Component%20Object%20Reference) (Depth :type Float%20%28single-precision%29))
  ;[1 1 1] Align Paper Sprite
  (Transformation|SetRelativeLocation Sprite (Math|Vector|MakeVector (.x (Transformation|GetWorldLocation Sprite)) Depth (.Z (Math|Vector|BreakVector (.BoxExtent (Collision|GetComponentBounds Sprite))))) false false))

(fn BindtoEvents
  ;[1 1 1] Bind to Events
  (bind _asbp_game_mode (Utilities|Casting|CastToBP_GameMode (Game|GetGameMode)))
  (EventDispatchers|BindEventtoGameStateChanged _asbp_game_mode (EventDispatchers|CreateEvent :!event OnGameStateChanged)))

(fn GetBaseNewLocation
  (params (Base :type Scene%20Component%20Object%20Reference) (DeltaSeconds :type Float%20%28single-precision%29))
  (bind _returnvalue (Transformation|GetWorldLocation Base))
  ;[1 1 1] Get Base New Location
  (return (Math|Vector|MakeVector (- (.x _returnvalue) (* DeltaSeconds (Variables|Default|Get_Speed))) (.y _returnvalue) (.z _returnvalue))))

(fn MoveBase
  (params (Base :type Scene%20Component%20Object%20Reference) (NextBase :type Scene%20Component%20Object%20Reference) (DeltaSeconds :type Float%20%28single-precision%29))
  ;[1 1 1] Move Base
  (Utilities|FlowControl|Sequence
    (:then_0
      (if (CallFunction|ShouldBaseRelocate Base)
        (CallFunction|RelocateBase Base NextBase)))
    (:then_1
      (Transformation|SetWorldLocation Base (CallFunction|GetBaseNewLocation Base DeltaSeconds) false false))))

(fn MoveBases
  (params (DeltaSeconds :type Float%20%28single-precision%29))
  ;[1 1 1] Move Bases
  (if (Variables|Default|Get_CanMove)
    (CallFunction|MoveBase (Variables|Default|GetBase01) (Variables|Default|GetBase02) DeltaSeconds)
    (CallFunction|MoveBase (Variables|Default|GetBase02) (Variables|Default|GetBase01) DeltaSeconds)))

(fn RelocateBase
  (params (Base :type Scene%20Component%20Object%20Reference) (RelocateAfterBase :type Scene%20Component%20Object%20Reference))
  (bind _returnvalue (Transformation|GetWorldLocation RelocateAfterBase))
  ;[1 1 1] Relocate Base
  (Transformation|SetWorldLocation Base (Math|Vector|MakeVector (+ (.x _returnvalue) (Variables|Default|Get_BaseWidth)) (.y _returnvalue) (.z _returnvalue)) false false))

(fn SetBaseWidth
  ;[1 1 1] Set Base Width
  (Variables|Default|Set_BaseWidth (* (.x (.BoxExtent (Collision|GetComponentBounds (Variables|Default|GetBase01)))) 2.0)))

(fn SetSpeed
  ;[1 1 1] Set Speed
  (bind _asbp_game_mode (Utilities|Casting|CastToBP_GameMode (Game|GetGameMode)))
  (Variables|Default|Set_Speed (Default|GetGameSpeed _asbp_game_mode)))

(fn ShouldBaseRelocate
  (params (Base :type Scene%20Component%20Object%20Reference))
  ;[1 1 1] Should Base Relocate?
  (return (<= (.x (Transformation|GetWorldLocation Base)) (- 0.0 (Variables|Default|Get_BaseWidth)))))

(fn SetRandomTimeOfDay
  ;[1 1 1] Set Random Time of Day
  (if (Variables|Default|Get_CanChangeBackground)
    (Rendering|Components|Sprite|SetSprite (Variables|Default|GetBackground) (select (Math|Random|RandomBool) "/Game/Environment/SPR_Background_Night.SPR_Background_Night" "/Game/Environment/SPR_Background_Day.SPR_Background_Day"))
    (Variables|Default|Set_CanChangeBackground false)))

(fn OnGameGetReady
  ;[1 1 1] Game - Get Ready
  (Variables|Default|Set_CanMove true)
  (CallFunction|SetRandomTimeOfDay))

(fn OnGameOver
  ;[1 1 1] Game - Over
  (Variables|Default|Set_CanMove false)
  (Variables|Default|Set_CanChangeBackground true))

(fn OnGamePlaying
  ;[1 1 1] Game - Playing
  (Variables|Default|Set_CanMove true))

(fn OnGameStarted
  ;[1 1 1] Game - Started
  (Variables|Default|Set_CanMove true)
  (CallFunction|SetRandomTimeOfDay))

(fn OnGameStateChanged
  (params (GameState :type EGameState%20Enum :default "NewEnumerator0"))
  ;[1 1 1] Game Start Changed
  (switch Utilities|FlowControl|Switch|SwitchonEGameState GameState
    (:NewEnumerator0
      (EventHandlers|OnGameStarted))
    (:NewEnumerator1
      (EventHandlers|OnGameGetReady))
    (:NewEnumerator2
      (EventHandlers|OnGamePlaying))
    (:NewEnumerator3
      (EventHandlers|OnGameOver))))